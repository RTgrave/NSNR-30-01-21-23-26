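; Networked character blueprint that can sprint, attack, and carry a book it drops on death.
; Sprint, attack and grab requests route to the server, which multicasts attack montages and times them.
; Server capsule overlaps set OverlapBook, whose RepNotify toggles the local interaction widget.
; HealthComponent events drive damage and death animations plus collision changes in Ragdoll, while Tick updates walk speed from sprint state.
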(event `self.ReceiveTick`
  (params (DeltaSeconds :type "Float (single-precision)"))
  (`self.UpdateSpeed`))

(event `self.HealthComponent.OnDamage`
  (params (Health :type "Float (single-precision)") (DamageCauser :type "Actor Object Reference"))
  ;[1 1 1] События Компонента Здоровья
  ;;[1 1 1] Урон персонажу
  (`self.PlayAnimMontage` (`self.AnimDamage`)))

(event `self.HealthComponent.OnDeath`
  (params (Causer :type "Actor Object Reference"))
  ;[1 1 1] События Компонента Здоровья
  ;;[1 1 1] Смерть персонажа
  (`SkeletalMeshComponent.PlayAnimation` (`self.Mesh`) (`self.AnimDeath`) false)
  (`self.Ragdoll`)
  (`self.DropBook`))

(event `self.CapsuleComponent.OnComponentBeginOverlap`
  (params (OverlappedComponent :type "PrimitiveComponent Object Reference") (OtherActor :type "Actor Object Reference") (OtherComp :type "PrimitiveComponent Object Reference") (OtherBodyIndex :type Integer) (bFromSweep :type Boolean) (SweepResult :type "HitResult Structure (by ref)"))
  ;[1 1 1] Обработка взаимодействия с книгой
  (`/Engine/EditorBlueprintResources/ActorMacros.Switch Has Authority`
    (:`Authority`
      (bind _asbp_book (cast `/Game/Blueprints/Game/BP_Book` OtherActor))
      (set `self.OverlapBook` _asbp_book))))

(event `self.CapsuleComponent.OnComponentEndOverlap`
  (params (OverlappedComponent :type "PrimitiveComponent Object Reference") (OtherActor :type "Actor Object Reference") (OtherComp :type "PrimitiveComponent Object Reference") (OtherBodyIndex :type Integer))
  ;[1 1 1] Обработка взаимодействия с книгой
  (`/Engine/EditorBlueprintResources/ActorMacros.Switch Has Authority`
    (:`Authority`
      (cast `/Game/Blueprints/Game/BP_Book` OtherActor)
      (set `self.OverlapBook` null))))

(event `self.ReceiveUnpossessed`
  (params (OldController :type "Controller Object Reference"))
  (`self.SetLifeSpan` 5.0))

(event `ServerAttack`
  (params (AnimAttack :type "AnimMontage Object Reference"))
  (`self.OnAttack` AnimAttack))

(event `MulticastAttack`
  (params (AnimAttack :type "AnimMontage Object Reference"))
  (`self.PlayAnimAttack` AnimAttack))

(event `ServerSetWantSprint`
  (params (WantSprint :type Boolean))
  (`self.SetWantSprint` WantSprint))

(event `ServerSetInteract`
  (`self.GrabBook`))

(event `ServerApplyDamage`
  (params (DamagedActor :type "Actor Object Reference") (BaseDamage :type "Float (double-precision)") (DamageTypeClass :type "DamageType Class Reference"))
  (`GameplayStatics.ApplyDamage` DamagedActor BaseDamage null self DamageTypeClass))

(fn `DropBook`
  (bind _book (`self.Book`))
  (`/Engine/EditorBlueprintResources/StandardMacros.IsValid` _book
    (:`Is Valid`
      (`/Game/Blueprints/Game/BP_Book.Drop` _book)
      (set `self.Book` null)
      (set `self.OverlapBook` null))))

(fn `GetAnimAttacking`
  (returns (ReturnValue :type "AnimMontage Object Reference"))
  (return (`|GetArrayItem` (`self.AttackAnimations`) (`KismetMathLibrary.RandomInteger` (`KismetArrayLibrary.Array_Length` (`self.AttackAnimations`))))))

(fn `GetBook`
  (returns (Book :type "/Game/Blueprints/Game/BP_Book Object Reference"))
  (return (`self.Book`)))

(fn `GrabBook`
  (`/Engine/EditorBlueprintResources/ActorMacros.Switch Has Authority`
    (:`Authority`
      (bind _overlapbook (`self.OverlapBook`)
        (:`then`
          (bind _output_get (set `self.Book` _overlapbook))
          (`/Game/Blueprints/Game/BP_Book.Grad` _output_get self))
        (:`else`)))
    (:`Remote`
      (`self.ServerSetInteract`))))

(fn `IsAttacting`
  (returns (IsAttacking :type Boolean))
  (return (`self.IsAttacking`)))

(fn `IsSprinting`
  (returns (ReturnValue :type Boolean))
  (bind _charactermovement (`self.CharacterMovement`))
  (return (and (`self.WantSprint`) (> (`KismetMathLibrary.VSize` (`self.GetVelocity`)) 0.0) (not (`NavMovementComponent.IsCrouching` _charactermovement)) (not (`NavMovementComponent.IsFalling` _charactermovement)))))

(fn `OnAttack`
  (params (AnimAttack :type "AnimMontage Object Reference"))
  (if (`self.IsAttacking`)
    (return)
    (else
      (set `self.IsAttacking` true)
      (`/Engine/EditorBlueprintResources/ActorMacros.Switch Has Authority`
        (:`Authority`
          (`self.MulticastAttack` AnimAttack))
        (:`Remote`
          (`self.ServerAttack` AnimAttack))))))

(fn `OnRep_OverlapBook`
  (bind _interactionwidget (`self.InteractionWidget`))
  (if (`self.IsLocallyControlled`)
    (`/Engine/EditorBlueprintResources/StandardMacros.IsValid` (`self.OverlapBook`)
      (:`Is Valid`
        (`/Engine/EditorBlueprintResources/StandardMacros.IsValid` _interactionwidget
          (:`Is Valid`
            _)
          (:`Is Not Valid`
            (bind _returnvalue (`|CreateWidget` "/Game/Widgets/WB_Interaction.WB_Interaction_C" (cast `PlayerController` (`self.GetController`) :!pure true)))
            (set `self.InteractionWidget` _returnvalue)))
        (`UserWidget.AddToPlayerScreen` _interactionwidget 0))
      (:`Is Not Valid`
        (`Widget.RemoveFromParent` _interactionwidget)))))

(fn `PlayAnimAttack`
  (params (AnimAttack :type "AnimMontage Object Reference"))
  (bind _returnvalue (`self.PlayAnimMontage` AnimAttack))
  (`/Engine/EditorBlueprintResources/ActorMacros.Switch Has Authority`
    (:`Authority`
      (bind _returnvalue_2 (`KismetSystemLibrary.K2_SetTimerDelegate` (`|CreateDelegate` :!event `StopAttack`) (/ _returnvalue 1.2)))
      (set `self.TH_Attack` _returnvalue_2))))

(fn `Ragdoll`
  (bind _charactermovement (`self.CharacterMovement`))
  (bind _capsulecomponent (`self.CapsuleComponent`))
  (`MovementComponent.StopMovementImmediately` _charactermovement)
  (`NavMovementComponent.StopMovementKeepPathing` _charactermovement)
  (`PrimitiveComponent.SetCollisionResponseToAllChannels` _capsulecomponent "ECR_Ignore")
  (`PrimitiveComponent.SetCollisionResponseToChannel` _capsulecomponent "ECC_WorldStatic" "ECR_Block")
  (`PrimitiveComponent.SetCollisionResponseToChannel` _capsulecomponent "ECC_WorldDynamic" "ECR_Block")
  (`PrimitiveComponent.SetCollisionObjectType` (`self.Mesh`) "ECC_PhysicsBody"))

(fn `SetWantSprint`
  (params (WantSprint :type Boolean))
  (set `self.WantSprint` WantSprint)
  (`/Engine/EditorBlueprintResources/ActorMacros.Switch Has Authority`
    (:`Remote`
      (`self.ServerSetWantSprint` WantSprint))))

(fn `StopAttack`
  (set `self.IsAttacking` false))

(fn `UpdateSpeed`
  (bind _charactermovement (`self.CharacterMovement`))
  (if (`self.IsSprinting`)
    (set `CharacterMovementComponent.MaxWalkSpeed` (`self.MaxSprintSpeed`) _charactermovement)
    (else
      (set `CharacterMovementComponent.MaxWalkSpeed` (`self.MaxWalkSpeed`) _charactermovement))))

(fn `UserConstructionScript`)