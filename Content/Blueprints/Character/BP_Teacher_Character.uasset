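; BP_Teacher_Character is a character Blueprint that maps player input to named attacks through OnAttack.
; A TripleTap macro counts presses in TimeAttacking and branches to single, double or triple after a 0.7-second Delay, without resetting counts above three.
; PrimaryAttack chains up to three timed attacks by tap count, while SecundaryAttack handles only single and double taps.
; Individual letter and numpad keys fire specific attacks directly.
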(event `InputAction|PrimaryAttack`
  (params (Key :type "Key Structure"))
  (:`Pressed`
    (`self.TripleTap`
      (:`Single`
        (`self.OnAttack` (`self.Primary`)))
      (:`Double`
        (`self.OnAttack` (`self.Primary`))
        (`KismetSystemLibrary.Delay` 1.0)
        (`self.OnAttack` (`self.Frank4-2`)))
      (:`Triple`
        (`self.OnAttack` (`self.Primary`))
        (`KismetSystemLibrary.Delay` 1.0)
        (`self.OnAttack` (`self.Frank4-2`))
        (`KismetSystemLibrary.Delay` 1.0)
        (`self.OnAttack` (`self.Frank4-3`))))))

(event `Key|Subtract`
  (params (Key :type "Key Structure"))
  (:`Pressed`
    (`self.OnAttack` (`self.Num-`))))

(event `InputAction|SecundaryAttack`
  (params (Key :type "Key Structure"))
  (:`Pressed`
    (`self.TripleTap`
      (:`Single`
        (`self.OnAttack` (`self.Y`)))
      (:`Double`
        (`self.OnAttack` (`self.P`))
        (`KismetSystemLibrary.Delay` 1.0)
        (`self.OnAttack` (`self.Attack kick 04`))))))

(event `Key|Multiply`
  (params (Key :type "Key Structure"))
  (:`Pressed`
    (`self.OnAttack` (`self.Num*`))))

(event `Key|Divide`
  (params (Key :type "Key Structure"))
  (:`Pressed`
    (`self.OnAttack` (`self.Num/`))))

(event `Key|T`
  (params (Key :type "Key Structure"))
  (:`Pressed`
    (`self.OnAttack` (`self.T`))))

(event `Key|Y`
  (params (Key :type "Key Structure"))
  (:`Pressed`
    (`self.OnAttack` (`self.Y`))))

(event `Key|U`
  (params (Key :type "Key Structure"))
  (:`Pressed`
    (`self.OnAttack` (`self.U`))))

(event `Key|I`
  (params (Key :type "Key Structure"))
  (:`Pressed`
    (`self.OnAttack` (`self.I`))))

(event `Key|O`
  (params (Key :type "Key Structure"))
  (:`Pressed`
    (`self.OnAttack` (`self.O`))))

(event `Key|P`
  (params (Key :type "Key Structure"))
  (:`Pressed`
    (`self.OnAttack` (`self.P`))))

(event `Key|G`
  (params (Key :type "Key Structure"))
  (:`Pressed`
    (`self.OnAttack` (`self.G`))))

(event `Key|H`
  (params (Key :type "Key Structure"))
  (:`Pressed`
    (`self.OnAttack` (`self.H`))))

(fn `UserConstructionScript`
  (`parent.UserConstructionScript`))