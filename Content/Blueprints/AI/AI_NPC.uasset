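; AI_NPC is an AI controller that runs the BT_NPC behavior tree and makes its NPC turn aggressive when damaged.
; On possess it binds to the pawn's HealthComponent damage and death events.
; Damage sets IsAgressive and stores the attacker in TargetAggressive, with an OnRep function copying the aggression flag to the Blackboard.
; Death unpossesses the pawn and stops movement.
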(event `self.ReceivePossess`
  (params (PossessedPawn :type "Pawn Object Reference"))
  (bind _returnvalue (`self.GetComponentByClass` PossessedPawn "/Game/Blueprints/Game/Components/HealthComponent.HealthComponent_C"))
  (`self.RunBehaviorTree` "/Game/Blueprints/AI/BT_NPC.BT_NPC")
  (`/Engine/EditorBlueprintResources/StandardMacros.IsValid` _returnvalue
    (:`Is Valid`
      (add `/Game/Blueprints/Game/Components/HealthComponent.OnDeath` _returnvalue (delegate `OnDeath_Event`))
      (add `/Game/Blueprints/Game/Components/HealthComponent.OnDamage` _returnvalue (delegate `OnDamage_Event`)))))

(event `OnDeath_Event`
  (params (Causer :type "Actor Object Reference"))
  (`self.UnPossess`)
  (`self.StopMovement`))

(event `OnDamage_Event`
  (params (Health :type "Float (double-precision)") (DamageCauser :type "Actor Object Reference"))
  (set `self.IsAgressive` true)
  (set `self.TargetAggressive ` DamageCauser))

(fn `OnRep_IsArgessia`
  (`BlackboardComponent.SetValueAsBool` (`self.Blackboard`) "IsAgressive" (`self.IsAgressive`)))

(fn `UserConstructionScript`)