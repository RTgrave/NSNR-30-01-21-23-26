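; Animation notify named Attack that performs a melee hit check when an attack animation reaches it.
; It runs a box trace at a socket on the mesh, sized and oriented by configurable hit box settings and ignoring the owner, with optional debug drawing.
; On a hit, it casts the owner to BP_SimpleCharacter and calls ServerApplyDamage on the hit actor with the configured damage and type.
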(fn `GetNotifyName`
  (returns (ReturnValue :type String))
  (return "Attack"))

(fn `Received_Notify`
  (params (MeshComp :type "SkeletalMeshComponent Object Reference") (Animation :type "AnimSequenceBase Object Reference"))
  (returns (ReturnValue :type Boolean))
  (bind _returnvalue (`ActorComponent.GetOwner` MeshComp))
  (bind (_returnvalue_location _returnvalue_rotation) (`KismetMathLibrary.BreakTransform` (`SceneComponent.GetSocketTransform` MeshComp (`self.SocketHitBox`) "RTS_World")))
  (bind (_outhit _returnvalue_2) (`KismetSystemLibrary.BoxTraceSingle` _returnvalue_location _returnvalue_location (`self.HitBoxSize`) _returnvalue_rotation "TraceTypeQuery3" true (`|MakeArray` _returnvalue) (`self.DrawDebugType`) true (`KismetMathLibrary.Conv_ColorToLinearColor` (`self.NotifyColor`)) (struct :`R` 1.0 :`A` 1.0) (`self.DrawBoxTime`)))
  (if _returnvalue_2
    (bind _asbp_simple_character (cast `/Game/Blueprints/Character/BP_SimpleCharacter` _returnvalue))
    (`/Game/Blueprints/Character/BP_SimpleCharacter.ServerApplyDamage` _asbp_simple_character (`.HitActor` (`GameplayStatics.BreakHitResult` _outhit)) (`self.Damage`) (`self.DamageType`))
    (return true)
    (else
      (return false))))