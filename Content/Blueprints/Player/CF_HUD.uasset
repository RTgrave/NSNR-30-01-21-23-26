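; The player HUD for a team match between Teachers and Students, which shows team selection and match results.
; On BeginPlay it shows the team choice widget, creating it only if none exists yet, and adds it to the player's screen.
; It also binds to the CF game state's end-match event and adds the Teacher or Student win widget to the viewport for the winning team.
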(event `self.ReceiveBeginPlay`
  ;[1 1 1] Создание меню выбора команды и привязка к событию окончания матча
  (`self.ShowTeamSelect`)
  (bind _ascf_game_state (cast `/Game/Blueprints/Online/CF_GameState` (`GameplayStatics.GetGameState`)))
  (add `/Game/Blueprints/Online/CF_GameState.OnEndMatch` _ascf_game_state (delegate `OnEndMatch_Event`)))

(event `OnEndMatch_Event`
  (params (Team :type "/Game/Blueprints/Game/ETeam Enum" :default "NewEnumerator2"))
  (bind _returnvalue (`self.GetOwningPlayerController`))
  ;[1 1 1] Создание меню выбора команды и привязка к событию окончания матча
  (switch `/Game/Blueprints/Game/ETeam` Team
    (:`NewEnumerator0`
      (bind _returnvalue_2 (`|CreateWidget` "/Game/Widgets/WB_TeamTeacherWin.WB_TeamTeacherWin_C" _returnvalue))
      (`UserWidget.AddToViewport` _returnvalue_2 0))
    (:`NewEnumerator1`
      (bind _returnvalue_3 (`|CreateWidget` "/Game/Widgets/WB_TeamStudentWin.WB_TeamStudentWin_C" _returnvalue))
      (`UserWidget.AddToViewport` _returnvalue_3 0))))

(fn `ShowTeamSelect`
  (`/Engine/EditorBlueprintResources/StandardMacros.IsValid` (`self.Team Choose Widget`)
    (:`Is Valid`
      _)
    (:`Is Not Valid`
      (bind _returnvalue (`|CreateWidget` "/Game/Widgets/WB_TeamChoose.WB_TeamChoose_C" (`self.GetOwningPlayerController`)))
      (set `self.Team Choose Widget` _returnvalue)))
  (`UserWidget.AddToPlayerScreen` (`self.Team Choose Widget`) 0)
  (return))

(fn `UserConstructionScript`)