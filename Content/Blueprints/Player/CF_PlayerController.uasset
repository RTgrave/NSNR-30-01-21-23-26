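; Player controller for the multiplayer CaptureBook mode, handling team selection, spawning and match flow.
; A tagged camera is the initial local view; SetTeam routes to the server, stores the team and spawns through the game mode.
; Pawn death unpossesses and reopens team selection; match end stops movement and unpossesses.
; On mode restart, client widgets are cleared, then players with teams respawn with HUD widgets while others see team selection.
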(event `self.ReceiveBeginPlay`
  ;[1 1 1] Привязка к стартовой камере и привязка к событию окончания матча, после окончания матча отключается перемещение персонажа и экшен кнопки
  (`self.StartCamera`)
  (`/Engine/EditorBlueprintResources/ActorMacros.Switch Has Authority`
    (:`Authority`
      (bind _ascf_game_state (cast `/Game/Blueprints/Online/CF_GameState` (`GameplayStatics.GetGameState`)))
      (add `/Game/Blueprints/Online/CF_GameState.OnEndMatch` _ascf_game_state (delegate `OnEndMatch_Event`))
      (bind _ascapture_book_game_mode (cast `/Game/Blueprints/Online/CaptureBook_GameMode` (`GameStateBase.AuthorityGameMode` (`GameplayStatics.GetGameState`))))
      (add `/Game/Blueprints/Online/CaptureBook_GameMode.OnRestartMode` _ascapture_book_game_mode (delegate `OnRestartMode_Event`)))))

(event `OnRestartMode_Event`
  ;[1 1 1] Привязка к стартовой камере и привязка к событию окончания матча, после окончания матча отключается перемещение персонажа и экшен кнопки
  (`self.ClientRemoveAllWidgets`)
  (if (`|EnumInequality` (`self.Team`) "NewEnumerator2")
    (`self.SpawnPlayerCharacter`)
    (else
      (`self.ClientShowTeamSelect`))))

(event `OnEndMatch_Event`
  (params (Team :type "/Game/Blueprints/Game/ETeam Enum" :default "NewEnumerator2"))
  (bind _returnvalue (`self.K2_GetPawn`))
  (bind _returnvalue_2 (`Pawn.GetMovementComponent` _returnvalue))
  ;[1 1 1] Привязка к стартовой камере и привязка к событию окончания матча, после окончания матча отключается перемещение персонажа и экшен кнопки
  (`/Engine/EditorBlueprintResources/StandardMacros.IsValid` _returnvalue
    (:`Is Valid`
      (`MovementComponent.StopMovementImmediately` _returnvalue_2)
      (`NavMovementComponent.StopMovementKeepPathing` _returnvalue_2)
      (`self.UnPossess`))))

(event `ClientRemoveAllWidgets`
  ;[1 1 1] Привязка к стартовой камере и привязка к событию окончания матча, после окончания матча отключается перемещение персонажа и экшен кнопки
  (`WidgetLayoutLibrary.RemoveAllWidgets`)
  (if (`|EnumInequality` (`self.Team`) "NewEnumerator2")
    (bind _returnvalue (`|CreateWidget` "/Game/Widgets/WB_GameText.WB_GameText_C" self))
    (`UserWidget.AddToViewport` _returnvalue 0)
    (bind _returnvalue_2 (`|CreateWidget` "/Game/Widgets/WB_Player_Health.WB_Player_Health_C" self))
    (`UserWidget.AddToPlayerScreen` _returnvalue_2 0)))

(event `ServerSetTeam`
  (params (Team :type "/Game/Blueprints/Game/ETeam Enum" :default "NewEnumerator2"))
  ;[0 0.15 0.1221] Выбор команды
  ;;[1 1 1] Вызов смены команды на сервере
  (`self.SetTeam` Team))

(event `ClientShowTeamSelect`
  ;[0 0.15 0.1221] Выбор команды
  ;;[1 1 1] Показать меню выбора команды на клиенте
  (bind _ascf_hud (cast `/Game/Blueprints/Player/CF_HUD` (`self.GetHUD`)))
  (`/Game/Blueprints/Player/CF_HUD.ShowTeamSelect` _ascf_hud))

(event `self.ReceivePossess`
  (params (PossessedPawn :type "Pawn Object Reference"))
  ;[1 1 1] При вселении контроллера в персонажа привязывется событие смерти после которогоконтроллер отключается от текущего персонажа и ожидает спан нового
  (`parent.ReceivePossess` PossessedPawn)
  (add `/Game/Blueprints/Game/Components/HealthComponent.OnDeath` (`self.GetComponentByClass` PossessedPawn "/Game/Blueprints/Game/Components/HealthComponent.HealthComponent_C") (delegate `OnDeath_Event`)))

(event `OnDeath_Event`
  (params (Causer :type "Actor Object Reference"))
  ;[1 1 1] При вселении контроллера в персонажа привязывется событие смерти после которогоконтроллер отключается от текущего персонажа и ожидает спан нового
  (`self.UnPossess`)
  (`self.ClientShowTeamSelect`))

(fn `SetTeam`
  (params (Team :type "/Game/Blueprints/Game/ETeam Enum" :default "NewEnumerator2"))
  (`/Engine/EditorBlueprintResources/ActorMacros.Switch Has Authority`
    (:`Authority`
      (set `self.Team` Team)
      (`self.SpawnPlayerCharacter`))
    (:`Remote`
      (`self.ServerSetTeam` Team))))

(fn `SpawnPlayerCharacter`
  (`GameModeBase.RestartPlayer` (`GameStateBase.AuthorityGameMode` (`GameplayStatics.GetGameState`)) self))

(fn `StartCamera`
  (if (`self.IsLocalController`)
    (bind _outactors (`GameplayStatics.GetAllActorsOfClassWithTag` "/Script/Engine.CameraActor" "SelectTeam"))
    (`self.SetViewTargetWithBlend` (`|GetArrayItem` _outactors))))

(fn `UserConstructionScript`)