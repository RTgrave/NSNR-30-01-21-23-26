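; Game mode for the team-based CaptureBook match, handling team spawning and the delayed restart after a match.
; It picks the Teacher or Student character from the controller's team, and players without a valid pawn class cannot restart.
; Spawning overrides the given transform with that of a random CustomPlayerStart tagged with the team name.
; The game state's end-match event starts a timer that then calls OnRestartMode.
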(event `self.ReceiveBeginPlay`
  ;[1 1 1] Привязка окончание матча и перезапуск игры
  (bind _ascf_game_state (cast `/Game/Blueprints/Online/CF_GameState` (`GameplayStatics.GetGameState`)))
  (add `/Game/Blueprints/Online/CF_GameState.OnEndMatch` _ascf_game_state (delegate `OnEndMatch_Event`)))

(event `OnEndMatch_Event`
  (params (Team :type "/Game/Blueprints/Game/ETeam Enum" :default "NewEnumerator2"))
  ;[1 1 1] Привязка окончание матча и перезапуск игры
  (`KismetSystemLibrary.K2_SetTimerDelegate` (delegate `RestartMatch`) (`self.TimeToRestart`)))

(event `RestartMatch`
  ;[1 1 1] Привязка окончание матча и перезапуск игры
  (`self.OnRestartMode`))

(fn `GetDefaultPawnClassForController`
  (params (InController :type "Controller Object Reference"))
  (returns (ReturnValue :type "Object Class Reference"))
  (bind _ascf_player_controller (cast `/Game/Blueprints/Player/CF_PlayerController` InController)
    (:`then`
      (switch `/Game/Blueprints/Game/ETeam` (`/Game/Blueprints/Player/CF_PlayerController.Team` _ascf_player_controller)
        (:`NewEnumerator2`
          (return null))
        (:`NewEnumerator0`
          (return "/Game/Blueprints/Character/BP_Teacher_Character.BP_Teacher_Character_C"))
        (:`NewEnumerator1`
          (return "/Game/Blueprints/Character/BP_Student_Character.BP_Student_Character_C"))))
    (:`CastFailed`
      (return null))))

(fn `GetPlayerStart`
  (params (Controller :type "Controller Object Reference"))
  (returns (PlayerStart :type "/Game/Blueprints/Game/CustomPlayerStart Object Reference"))
  (bind _ascf_player_controller (cast `/Game/Blueprints/Player/CF_PlayerController` Controller))
  (bind _outactors (`GameplayStatics.GetAllActorsOfClassWithTag` "/Game/Blueprints/Game/CustomPlayerStart.CustomPlayerStart_C" (`KismetStringLibrary.Conv_StringToName` (`|GetEnumeratorNameAsString` (`/Game/Blueprints/Player/CF_PlayerController.Team` _ascf_player_controller)))))
  (return (`|GetArrayItem` _outactors (`KismetMathLibrary.RandomInteger` (`KismetArrayLibrary.Array_LastIndex` _outactors)))))

(fn `PlayerCanRestart`
  (params (Player :type "PlayerController Object Reference"))
  (returns (ReturnValue :type Boolean))
  (bind _returnvalue (`self.GetDefaultPawnClassForController` Player))
  (return (`KismetSystemLibrary.IsValidClass` _returnvalue)))

(fn `SpawnDefaultPawnAtTransform`
  (params (NewPlayer :type "Controller Object Reference") (SpawnTransform :type "Transform Structure (by ref)"))
  (returns (ReturnValue :type "Pawn Object Reference"))
  (bind _playerstart (`self.GetPlayerStart` NewPlayer))
  (bind _returnvalue (`parent.SpawnDefaultPawnAtTransform` NewPlayer (`self.GetTransform` _playerstart)))
  (return _returnvalue))

(fn `UserConstructionScript`)