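; BP_Book is a carriable book actor that Teacher and Student teams can take and drop.
; Grad hides it and calls MulticastGrab, which disables collision, attaches it to the taker and shows a team-specific pickup widget.
; Drop calls MulticastDrop to detach it and restore query collision, then clears the owner and unhides it.
; UpdateBookLocation, run within MulticastDrop, snaps an unowned book to a line-trace hit toward world point Z -1000.
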(event `MulticastGrab`
  (params (ParentActor :type "Actor Object Reference") (Team :type "/Game/Blueprints/Game/ETeam Enum" :default "NewEnumerator2"))
  ;[1 1 1] Визуальное отображение взятия книги и оповещение всем игрокам о том какая команда взяла книгу
  (`PrimitiveComponent.SetCollisionEnabled` (`self.Box`) "NoCollision")
  (`PrimitiveComponent.SetCollisionEnabled` (`self.StaticMesh`) "NoCollision")
  (`self.K2_AttachToActor` ParentActor "None" "SnapToTarget" "SnapToTarget" "SnapToTarget")
  (switch `/Game/Blueprints/Game/ETeam` Team
    (:`NewEnumerator0`
      (bind _returnvalue (`|CreateWidget` "/Game/Widgets/WB_TeamTeacherTakeBook.WB_TeamTeacherTakeBook_C"))
      (`UserWidget.AddToViewport` _returnvalue 0))
    (:`NewEnumerator1`
      (bind _returnvalue_2 (`|CreateWidget` "/Game/Widgets/WB_TeamStudentTakeBook.WB_TeamStudentTakeBook_C"))
      (`UserWidget.AddToViewport` _returnvalue_2 0))))

(event `MulticastDrop`
  ;[1 1 1] Визуальное отображение сброса книги владельцем
  (`self.K2_DetachFromActor` "KeepWorld" "KeepWorld" "KeepWorld")
  (`PrimitiveComponent.SetCollisionEnabled` (`self.Box`) "QueryOnly")
  (`PrimitiveComponent.SetCollisionEnabled` (`self.StaticMesh`) "QueryOnly")
  (`self.UpdateBookLocation`))

(fn `Drop`
  (`self.MulticastDrop`)
  (`self.SetOwner` null)
  (`self.SetActorHiddenInGame` false))

(fn `Grad`
  (params (NewOwner :type "Actor Object Reference"))
  (`self.SetActorHiddenInGame` true)
  (bind _ascf_player_controller (cast `/Game/Blueprints/Player/CF_PlayerController` (`self.GetInstigatorController` NewOwner)))
  (`self.MulticastGrab` NewOwner (`/Game/Blueprints/Player/CF_PlayerController.Team` _ascf_player_controller)))

(fn `UpdateBookLocation`
  (`/Engine/EditorBlueprintResources/StandardMacros.IsValid` (`self.GetOwner`)
    (:`Is Valid`
      (return))
    (:`Is Not Valid`
      (bind (_outhit _returnvalue) (`KismetSystemLibrary.LineTraceSingleForObjects` (`self.K2_GetActorLocation`) (0.0 0.0 -1000.0) (`|MakeArray` "ObjectTypeQuery1" "ObjectTypeQuery2" "ObjectTypeQuery4" :!type "EObjectTypeQuery Enum") true))
      (if _returnvalue
        (`self.K2_SetActorLocation` (`.Location` (`GameplayStatics.BreakHitResult` _outhit)))))))

(fn `UserConstructionScript`)