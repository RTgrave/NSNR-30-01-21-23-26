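; BP_WinPlaceTeam is a team-specific win zone that ends the match when a player from its team brings the book to it.
; On collision overlap, it casts the instigator controller to CF_PlayerController and compares that player's Team with its own.
; If they match and the overlapping BP_SimpleCharacter holds a valid book, it calls CallWin with the team.
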(event `self.CollisionComponent.OnComponentBeginOverlap`
  (params (OverlappedComponent :type "PrimitiveComponent Object Reference") (OtherActor :type "Actor Object Reference") (OtherComp :type "PrimitiveComponent Object Reference") (OtherBodyIndex :type Integer) (bFromSweep :type Boolean) (SweepResult :type "HitResult Structure (by ref)"))
  ;[1 1 1] Если игрок с книгой из соответствующей команды взаимодействует то происходит вызов окончания матча
  (bind _ascf_player_controller (cast `/Game/Blueprints/Player/CF_PlayerController` (`self.GetInstigatorController` OtherActor)))
  (if (`|EnumEquality` (`/Game/Blueprints/Player/CF_PlayerController.Team` _ascf_player_controller) (`self.Team`))
    (bind _asbp_simple_character (cast `/Game/Blueprints/Character/BP_SimpleCharacter` OtherActor))
    (`/Engine/EditorBlueprintResources/StandardMacros.IsValid` (`/Game/Blueprints/Character/BP_SimpleCharacter.GetBook` _asbp_simple_character)
      (:`Is Valid`
        (`self.Win` (`self.Team`))))))

(fn `UserConstructionScript`)